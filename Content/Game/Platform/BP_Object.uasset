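; BP_Object is a world object with a static mesh, a hint component and a target socket name exposed through a getter.
; On BeginPlay it caches the third-person game mode and overrides the mesh's mass with that mode's default object weight.
; The construction script stores the hint root's initial relative location.
; Hit-based character impulse and mass-scale logic remain in the graph but are disconnected.
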(event `self.ReceiveBeginPlay`
  (bind _asbp_third_person_game_mode (cast `/Game/ThirdPerson/Blueprints/BP_ThirdPersonGameMode` (`GameplayStatics.GetGameMode`)))
  (set `self.GameMode` _asbp_third_person_game_mode)
  (`PrimitiveComponent.SetMassOverrideInKg` (`self.StaticMesh`) "None" (`self.GetWeight`) true))

(event `self.StaticMesh.OnComponentHit`
  (params (HitComponent :type "PrimitiveComponent Object Reference") (OtherActor :type "Actor Object Reference") (OtherComp :type "PrimitiveComponent Object Reference") (NormalImpulse :type "Vector Structure") (Hit :type "HitResult Structure (by ref)")))

(fn `GetTargetSocketName`
  (returns (SnapBoneName :type Name))
  (return (`self.TargetSocketName`)))

(fn `GetWeight`
  (returns (DefaultObjectWeight :type "Float (double-precision)"))
  (return (`/Game/ThirdPerson/Blueprints/BP_ThirdPersonGameMode.DefaultObjectWeight` (`self.GameMode`))))

(fn `UserConstructionScript`
  (set `self.InitialHintRelativeLocation` (`SceneComponent.RelativeLocation` (`self.HintRoot`))))