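; Object spawner actor that drops randomly chosen classes from a list at random points inside its bounds box, sampled at half the box extent.
; Each spawned object's static mesh receives a random-strength impulse within a cone around the fall direction.
; With auto-spawn on, a looping timer started at BeginPlay drives spawning.
; Debug keys spawn one object (Y) or toggle pausing the timer (P).
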(event Custom|SpawnRandomObject
  (bind _bounds (Variables|Default|GetBounds))
  (bind _objectclasstospawn (Variables|Default|GetObjectClassToSpawn))
  (bind _returnvalue (Game|SpawnActorfromClass (Utilities|Array|Get(acopy) _objectclasstospawn (.OutIndex (Utilities|Array|Random _objectclasstospawn))) (Math|Conversions|ToTransform(Vector) (Math|Random|RandomPointinBoundingBox (Transformation|GetWorldLocation _bounds) (* (Variables|/Script/Engine.BoxComponent|GetBoxExtent _bounds) 0.5))) "Undefined" "MultiplyWithRoot" 0 0))
  (Physics|AddImpulse (Variables|/Game/Game/Platform/BP_Object.BP_Object_C|GetStaticMesh _returnvalue) (* (Math|Random|RandomUnitVectorinConeinDegrees (Math|Vector|GetForwardVector (Variables|Default|GetFallDirection)) (Variables|Default|GetCone%20Half%20Angle%20in%20Degrees)) (Math|Random|RandomFloatinRange (Variables|Default|GetMinRandomImpulse) (Variables|Default|GetMaxRandomImpulse))) "None" false))

(event EventBeginPlay
  (if (Variables|Default|GetAutoSpawn)
    (bind _returnvalue (Utilities|Time|SetTimerbyEvent (delegate Custom|SpawnRandomObject) (Variables|Default|GetSpawnRate) true))
    (Variables|Default|SetTimerHandle _returnvalue)))

(event Input|KeyboardEvents|DebugKeyP
  (params (Key :type Key%20Structure :default "None") (ActionValue :type Input%20Action%20Value%20Structure))
  (:Pressed
    (Utilities|FlowControl|FlipFlop
      (:A
        (Utilities|Time|PauseTimerbyHandle (Variables|Default|GetTimerHandle))
        (Development|PrintString "Paused object spawner."))
      (:B
        (Utilities|Time|UnpauseTimerbyHandle (Variables|Default|GetTimerHandle))
        (Development|PrintString "UnPaused object spawner. ")))))

(event Input|KeyboardEvents|DebugKeyY
  (params (Key :type Key%20Structure :default "None") (ActionValue :type Input%20Action%20Value%20Structure))
  (:Pressed
    (CallFunction|SpawnRandomObject)))

(fn ConstructionScript)