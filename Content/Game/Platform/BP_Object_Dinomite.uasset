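; Dinomite is a throwable explosive object that starts a 2D fuse sound on spawn and detonates when its fuse runs out.
; Tick steadily lowers StaticMesh1's relative Z as the countdown, triggering a one-time explosion once it reaches zero.
; Detonation fires a radial force impulse, plays the SoundManager explosion, makes any character holding it throw it, stops the fuse sound and destroys the actor.
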(event `self.ReceiveBeginPlay`
  (`parent.ReceiveBeginPlay`)
  (bind _returnvalue (`GameplayStatics.SpawnSound2D` "/Game/Game/sound/fuse.fuse" 1.0 1.0 0.0 null))
  (set `self.FuseSound` _returnvalue))

(event `self.ReceiveTick`
  (params (DeltaSeconds :type "Float (single-precision)"))
  (bind _staticmesh1 (`self.StaticMesh1`))
  (bind (_relativelocation_x _relativelocation_y _relativelocation_z) (`KismetMathLibrary.BreakVector` (`SceneComponent.RelativeLocation` _staticmesh1)))
  (bind _returnvalue (- _relativelocation_z (* DeltaSeconds 5.0)))
  (`parent.ReceiveTick` DeltaSeconds)
  (`SceneComponent.K2_SetRelativeLocation` _staticmesh1 (`KismetMathLibrary.MakeVector` 0.0 0.0 _returnvalue) false false)
  (if (<= _returnvalue 0.0)
    (`/Engine/EditorBlueprintResources/StandardMacros.DoOnce` false
      (:`Completed`
        (`RadialForceComponent.FireImpulse` (`self.RadialForce`))
        (bind _returnvalue_2 (`GameplayStatics.GetActorOfClass` "/Game/Game/sound/SoundManager.SoundManager_C"))
        (`/Game/Game/sound/SoundManager.PlayExplosion` _returnvalue_2)
        (bind _outactors (`GameplayStatics.GetAllActorsOfClass` "/Game/ThirdPerson/Blueprints/BP_ThirdPersonCharacter.BP_ThirdPersonCharacter_C"))
        (for _array_element _outactors
          (if (== (`/Game/ThirdPerson/Blueprints/BP_ThirdPersonCharacter.PickedUpObject` _array_element) self)
            (`/Game/ThirdPerson/Blueprints/BP_ThirdPersonCharacter.ThrowObject` _array_element)))
        (`ActorComponent.SetActive` (`self.FuseSound`) false false)
        (`ActorComponent.K2_DestroyComponent` (`self.FuseSound`))
        (`self.K2_DestroyActor`)))))

(fn `UserConstructionScript`
  (`parent.UserConstructionScript`))