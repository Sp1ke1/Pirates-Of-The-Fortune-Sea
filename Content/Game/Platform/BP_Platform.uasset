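; BP_Platform is a tilting platform with gold collection zones for two players that ends the game when it tips to its rotation limit.
; On BeginPlay it assigns player indices to the BP_GoldCollector child actors in both zones.
; AddDeltaRotation adds roll to RotationRoot, clamped to MaxRotation, and calls EndGame on BP_God once at either limit.
; ResetRotation levels the root, and two debug keys tilt it in opposite directions.
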(event Custom|AddDeltaRotation
  (params (Angle :type Float%20%28double-precision%29))
  (bind _maxrotation (Variables|Default|GetMaxRotation))
  (bind _rotationroot (Variables|Default|GetRotationRoot))
  (bind _rotationroot_2 (Variables|Default|GetRotationRoot))
  (bind _returnvalue (* _maxrotation -1.0))
  (bind _relativerotation (Variables|/Script/Engine.SceneComponent|GetRelativeRotation _rotationroot))
  (bind _relativerotation_2 (Variables|/Script/Engine.SceneComponent|GetRelativeRotation _rotationroot_2))
  (bind _returnvalue_2 (+ Angle (.roll _relativerotation)))
  (bind _returnvalue_3 (Math|Float|Clamp(Float) _returnvalue_2 _returnvalue _maxrotation))
  (Transformation|SetRelativeRotation (Variables|Default|GetRotationRoot) (Math|Rotator|MakeRotator _returnvalue_3 (.pitch _relativerotation_2) (.yaw _relativerotation_2)) false false)
  (if (>= (Math|Float|Absolute(Float) _returnvalue_3) (Variables|Default|GetMaxRotation))
    (Utilities|FlowControl|DoOnce false
      (:Completed
        (bind _returnvalue_4 (Actor|GetActorOfClass "/Game/ThirdPerson/Blueprints/BP_God.BP_God_C"))
        (Default|EndGame _returnvalue_4 false)))))

(event Custom|ResetRotation
  (Transformation|SetRelativeRotation (Variables|Default|GetRotationRoot) "0, 0, 0" false false))

(event EventBeginPlay
  (bind _asbp_gold_collector (Utilities|Casting|CastToBP_GoldCollector (Variables|/Script/Engine.ChildActorComponent|GetChildActor (Variables|Default|GetPlayerZone1))))
  (Variables|/Game/Game/blueprints/BP_GoldCollector.BP_GoldCollector_C|SetPlayerIndex _asbp_gold_collector 0)
  (bind _asbp_gold_collector_2 (Utilities|Casting|CastToBP_GoldCollector (Variables|/Script/Engine.ChildActorComponent|GetChildActor (Variables|Default|GetPlayerZone2))))
  (Variables|/Game/Game/blueprints/BP_GoldCollector.BP_GoldCollector_C|SetPlayerIndex _asbp_gold_collector_2 1))

(event Input|KeyboardEvents|DebugKeyJ
  (params (Key :type Key%20Structure :default "None") (ActionValue :type Input%20Action%20Value%20Structure))
  (:Pressed
    (CallFunction|AddDeltaRotation (* (Variables|Default|GetDefaultDeltaAngle) -1.0))))

(event Input|KeyboardEvents|DebugKeyH
  (params (Key :type Key%20Structure :default "None") (ActionValue :type Input%20Action%20Value%20Structure))
  (:Pressed
    (CallFunction|AddDeltaRotation (Variables|Default|GetDefaultDeltaAngle))))

(fn ConstructionScript)