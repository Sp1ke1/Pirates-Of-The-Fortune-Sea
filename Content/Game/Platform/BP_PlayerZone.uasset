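; BP_PlayerZone is a zone that tilts the level's platform according to the mass of actors inside its box.
; Each tick it re-sums the mass of tagged overlapping actors and rotates the platform by that total, with a configurable multiplier and direction.
; Mass comes from simulating primitives, or the pelvis bone for non-simulating skeletal meshes.
; Incremental add/remove functions also exist, though this graph never calls them.
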(event `self.ReceiveBeginPlay`
  (`parent.ReceiveBeginPlay`)
  (bind _outactors (`GameplayStatics.GetAllActorsOfClass` (`self.PlatformClass`)))
  (if (`KismetArrayLibrary.Array_IsValidIndex` _outactors)
    (set `self.Platform` (`|GetArrayItem` _outactors))
    (else
      (`KismetSystemLibrary.PrintString` "Platform wasn't found!")
      (`self.K2_DestroyActor`))))

(event `self.ReceiveTick`
  (params (DeltaSeconds :type "Float (single-precision)"))
  (`parent.ReceiveTick` DeltaSeconds)
  (`self.UpdateMass`)
  (if (> (`self.TotalMassInBounds`) 0.0)
    (bind _platform (`self.Platform`)
      (:`then`
        (`/Game/Game/Platform/BP_Platform.AddDeltaRotation` _platform (* (`self.TotalMassInBounds`) DeltaSeconds (`self.MassToRotationMultiplier`) (`KismetMathLibrary.SelectFloat` -1.0 1.0 (`self.NegateRotationDirection`)))))
      (:`else`))))

(fn `AddOverlappingObject`
  (params (Actor :type "Actor Object Reference"))
  (if (not (`BlueprintSetLibrary.Set_Contains` (`self.OverlappingObjects`) Actor))
    (set `self.TotalMassInBounds` (+ (`self.TotalMassInBounds`) (`self.GetActorMass` Actor)))
    (`BlueprintSetLibrary.Set_Add` (`self.OverlappingObjects`) Actor)
    (`KismetSystemLibrary.PrintString` (`KismetStringLibrary.Concat_StrStr` " Added: " (`KismetSystemLibrary.GetDisplayName` Actor) " for player zone: " (`KismetStringLibrary.Conv_IntToString` (`self.ZoneIndex`)) " total mass: " (`KismetStringLibrary.Conv_DoubleToString` (`self.TotalMassInBounds`))))))

(fn `GetActorMass`
  (params (Actor :type "Actor Object Reference"))
  (returns (OutMass :type "Float (single-precision)"))
  (locals (Mass :type "Float (single-precision)" :default 0.0))
  (if (`self.ActorHasTag` Actor (`self.MassTag`))
    (for _array_element (`self.K2_GetComponentsByClass` Actor "/Script/Engine.PrimitiveComponent")
      (if (`SceneComponent.IsSimulatingPhysics` _array_element "None")
        (set `local.Mass` (+ (`PrimitiveComponent.GetMass` _array_element) (`local.Mass`)))
        (else
          (bind _asskeletal_mesh_component (cast `SkeletalMeshComponent` _array_element))
          (set `local.Mass` (+ (`SkeletalMeshComponent.GetBoneMass` _asskeletal_mesh_component "pelvis" false) (`local.Mass`))))))
    (return (`local.Mass`))))

(fn `RemoveOverlappingObject`
  (params (Actor :type "Actor Object Reference"))
  (if (`BlueprintSetLibrary.Set_Contains` (`self.OverlappingObjects`) Actor)
    (`|ExecutionSequence`
      (:`then_0`
        (set `self.TotalMassInBounds` (- (`self.TotalMassInBounds`) (`self.GetActorMass` Actor))))
      (:`then_1`
        (`BlueprintSetLibrary.Set_Remove` (`self.OverlappingObjects`) Actor)
        (`KismetSystemLibrary.PrintString` (`KismetStringLibrary.Concat_StrStr` " Removed: " (`KismetSystemLibrary.GetDisplayName` Actor) " from player zone: " (`KismetStringLibrary.Conv_IntToString` (`self.ZoneIndex`)) " total mass: " (`KismetStringLibrary.Conv_DoubleToString` (`self.TotalMassInBounds`))))))))

(fn `UpdateMass`
  (set `self.TotalMassInBounds` 0.0)
  (for _array_element (`PrimitiveComponent.GetOverlappingActors` (`self.Box`) "/Script/Engine.Actor")
    (set `self.TotalMassInBounds` (+ (`self.GetActorMass` _array_element) (`self.TotalMassInBounds`)))))

(fn `UserConstructionScript`)