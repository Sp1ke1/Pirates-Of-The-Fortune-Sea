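; BP_RespawnPlane is a trigger plane that respawns player characters and cleans up objects that overlap it.
; On BeginPlay it caches the platform actor found by class, which supplies a respawn point for each of the two players.
; Overlapping third-person characters teleport to the point selected by their PlayerIndex, taking its location and rotation.
; Overlapping BP_Object actors are destroyed after a configurable delay.
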(event `self.ReceiveBeginPlay`
  (bind _returnvalue (`GameplayStatics.GetActorOfClass` (`self.PlatformClass`)))
  (`/Engine/EditorBlueprintResources/StandardMacros.IsValid` _returnvalue
    (:`Is Valid`
      (set `self.Platform` _returnvalue))
    (:`Is Not Valid`
      (`KismetSystemLibrary.PrintString` "Platform is not valid"))))

(event `self.Box.OnComponentBeginOverlap`
  (params (OverlappedComponent :type "PrimitiveComponent Object Reference") (OtherActor :type "Actor Object Reference") (OtherComp :type "PrimitiveComponent Object Reference") (OtherBodyIndex :type Integer) (bFromSweep :type Boolean) (SweepResult :type "HitResult Structure (by ref)"))
  (bind _platform (`self.Platform`))
  (bind _asbp_third_person_character (cast `/Game/ThirdPerson/Blueprints/BP_ThirdPersonCharacter` OtherActor)
    (:`then`
      (bind _playerindex (`/Game/ThirdPerson/Blueprints/BP_ThirdPersonCharacter.PlayerIndex` _asbp_third_person_character))
      (`self.K2_SetActorLocationAndRotation` _asbp_third_person_character (.location (`SceneComponent.K2_GetComponentToWorld` (select `int` _playerindex :`0` (`/Game/Game/Platform/BP_Platform.PlayerRespawn1` _platform) :`1` (`/Game/Game/Platform/BP_Platform.PlayerRespawn2` _platform)))) (.rotation (`SceneComponent.K2_GetComponentToWorld` (select `int` _playerindex :`0` (`/Game/Game/Platform/BP_Platform.PlayerRespawn1` _platform) :`1` (`/Game/Game/Platform/BP_Platform.PlayerRespawn2` _platform)))) false true)
      (`KismetSystemLibrary.PrintString` (`KismetStringLibrary.Concat_StrStr` "Respawned character: " (`KismetStringLibrary.Conv_IntToString` _playerindex))))
    (:`CastFailed`
      (bind _asbp_object (cast `/Game/Game/Platform/BP_Object` OtherActor))
      (`KismetSystemLibrary.Delay` (`self.ObjectDestroyDelay`))
      (`/Engine/EditorBlueprintResources/StandardMacros.IsValid` _asbp_object
        (:`Is Valid`
          (`self.K2_DestroyActor` _asbp_object))))))

(fn `UserConstructionScript`)