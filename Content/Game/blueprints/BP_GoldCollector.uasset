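; Gold collector actor that builds up a gold total from the BP_GoldObject actors overlapping its box and displays it on a text render.
; While ShouldCount is true, each Tick sums their costs via GetGoldCount, scales the sum by the game mode's GoldSpeedScale and adds it to CurrentGold.
; The increment is per frame, without delta time.
; GetGoldAmount is an older variant that the event graph never runs.
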(event `self.ReceiveBeginPlay`
  (bind _asbp_third_person_game_mode (cast `/Game/ThirdPerson/Blueprints/BP_ThirdPersonGameMode` (`GameplayStatics.GetGameMode`)))
  (set `self.GameMode` _asbp_third_person_game_mode))

(event `self.ReceiveTick`
  (params (DeltaSeconds :type "Float (single-precision)"))
  (if (`self.bShouldCount`)
    (bind _goldamount (`self.GetGoldCount`))
    (set `self.CurrentGold` (+ (* _goldamount (`/Game/ThirdPerson/Blueprints/BP_ThirdPersonGameMode.GoldSpeedScale` (`self.GameMode`))) (`self.CurrentGold`)))
    (`TextRenderComponent.K2_SetText` (`self.TextRender`) (`KismetTextLibrary.Conv_StringToText` (`KismetStringLibrary.Concat_StrStr` "GOLD: " (`KismetTextLibrary.Conv_TextToString` (`KismetTextLibrary.Conv_DoubleToText` (`self.CurrentGold`) "HalfToEven" false true 1 324 1 1)))))))

(fn `GetGoldAmount`
  (returns (GoldAmount :type "Float (double-precision)"))
  (locals (GatheredGoldAmount :type "Float (double-precision)" :default 0.0))
  (for _array_element (`PrimitiveComponent.GetOverlappingActors` (`self.Box`) "/Game/Game/Platform/Objects/BP_GoldObject.BP_GoldObject_C")
    (bind _asbp_gold_object (cast `/Game/Game/Platform/Objects/BP_GoldObject` _array_element))
    (set `local.GatheredGoldAmount` (+ (`/Game/Game/Platform/Objects/BP_GoldObject.Cost` _asbp_gold_object) (`local.GatheredGoldAmount`))))
  (`TextRenderComponent.K2_SetText` (`self.TextRender`) (`KismetTextLibrary.Conv_StringToText` (`KismetStringLibrary.Concat_StrStr` "GOLD: " (`KismetStringLibrary.Conv_DoubleToString` (`local.GatheredGoldAmount`)))))
  (return (`local.GatheredGoldAmount`)))

(fn `GetGoldCount`
  (returns (GoldAmount :type "Float (double-precision)"))
  (locals (GatheredGoldAmount :type "Float (double-precision)" :default 0.0))
  (for _array_element (`PrimitiveComponent.GetOverlappingActors` (`self.Box`) "/Game/Game/Platform/Objects/BP_GoldObject.BP_GoldObject_C")
    (bind _asbp_gold_object (cast `/Game/Game/Platform/Objects/BP_GoldObject` _array_element))
    (bind _goldcost (`/Game/Game/Platform/Objects/BP_GoldObject.GetCost` _asbp_gold_object))
    (set `local.GatheredGoldAmount` (+ _goldcost (`local.GatheredGoldAmount`))))
  (return (`local.GatheredGoldAmount`)))

(fn `UserConstructionScript`)