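; Actor component that applies character customization items, swapping the main skeletal mesh or the hat static mesh.
; ApplyItem switches on slot type, async-loads the item's asset, then casts and sets it through the ApplySkeletalMesh and ApplyStaticMesh helpers.
; Hats are also snapped to the main mesh's "hatSocket".
; ApplyPreset is empty; a loop over preset slots remains in the graph but is disconnected.
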(event `self.ApplyPreset`
  (params (Preset :type "CharacterPresetRecord Structure (by ref)")))

(event `self.ApplyItem`
  (params (Item :type "CustomizationSlotItem Structure (by ref)") (SlotIndex :type Integer))
  (bind (_displayname _slottype _mesh _staticmesh) (break `CustomizationSlotItem` Item))
  (bind _hatmeshcomponent (`self.HatMeshComponent`))
  (switch `ECustomizationSlotType` _slottype
    (:`MainMesh`
      (bind _object (`|LoadAsset` _mesh)
        (:`Completed`
          (`self.ApplySkeletalMesh` _object (`self.MainMeshComponent`)))))
    (:`Hat`
      (bind _object_2 (`|LoadAsset` _staticmesh)
        (:`Completed`
          (`self.ApplyStaticMesh` _object_2 _hatmeshcomponent)
          (`SceneComponent.K2_AttachToComponent` _hatmeshcomponent (`self.MainMeshComponent`) "hatSocket" "SnapToTarget" "SnapToTarget" "SnapToTarget" true))))))

(fn `ApplySkeletalMesh`
  (params (Object :type "Object Object Reference") (SkeletalMesh :type "SkeletalMeshComponent Object Reference"))
  (bind _asskeletal_mesh (cast `SkeletalMesh` Object))
  (set `SkeletalMeshComponent.SkeletalMeshAsset` _asskeletal_mesh SkeletalMesh))

(fn `ApplyStaticMesh`
  (params (Object :type "Object Object Reference") (StaticMesh :type "StaticMeshComponent Object Reference"))
  (bind _asstatic_mesh (cast `StaticMesh` Object))
  (`StaticMeshComponent.SetStaticMesh` StaticMesh _asstatic_mesh))