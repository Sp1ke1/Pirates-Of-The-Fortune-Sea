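; Post-process actor that draws configurable outlines on custom-stencil ranges, part of the Stylized Rendering System for Mobile.
; Refresh, run from the construction script, clears the post-process materials, caps OutlineTypes at 25, and sets the volume unbound or box-bounded.
; Each visible type gets a dynamic material instance for color, thickness, occlusion visibility and distance fade/scale.
; Separate parent materials per index, with differing blendable priorities, let multiple outlines render simultaneously.
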(fn `Refresh`
  (bind _postprocess (`self.PostProcess`))
  (bind _outline_types (`self.Outline Types`))
  (bind _box (`self.Box`))
  ;[1 1 1] Reset Post Process Volume in case this method is executed manually
  (`KismetArrayLibrary.Array_Clear` (`.Array` (break `WeightedBlendables` (`.WeightedBlendables` (break `PostProcessSettings` (`PostProcessComponent.Settings` (`self.PostProcess`)))))))
  ;[1 1 1] Max Outline Number Cap
  (for _ (range 25 (+ (`KismetArrayLibrary.Array_Length` _outline_types) 1))
    (`KismetArrayLibrary.Array_Remove` _outline_types 25))
  (if (`self.Enable Outlines`)
    ;[1 1 1] Limited to Bounds
    (if (`self.Limited to Bounds`)
      (`SceneComponent.SetVisibility` _box true false)
      (set `PostProcessComponent.bUnbound` false _postprocess)
      (`BoxComponent.SetBoxExtent` _box (`self.Bounds`) true)
      (else
        (`SceneComponent.SetVisibility` _box false false)
        (set `PostProcessComponent.bUnbound` true _postprocess)))
    ;[1 1 1] Outlines
    (for (_array_element _array_index) (`self.Outline Types`)
      (bind ((`VisiblewheninLineofSight_23_0749EA41454B5BB2A02396A59F31B971` _visiblewheninlineofsight) (`Visiblewhenobstructed_25_475C2BDA4D5092C69A9DAD967937B2EC` _visiblewhenobstructed)) (break `/Game/StylizedRenderingSystemForMobile/Blueprints/Structs/BP_SRS_Outline_Struct` _array_element))
      ;;[1 1 1] Only Enable Outline Post Process if it is visible
      (if (or _visiblewheninlineofsight _visiblewhenobstructed)
        (bind _returnvalue (`KismetMaterialLibrary.CreateDynamicMaterialInstance` (select `int` _array_index :`0` "/Game/StylizedRenderingSystemForMobile/Materials/Private/PostProcessOutlines/M_SRS_Outline01.M_SRS_Outline01" :`1` "/Game/StylizedRenderingSystemForMobile/Materials/Private/PostProcessOutlines/M_SRS_Outline02.M_SRS_Outline02" :`2` "/Game/StylizedRenderingSystemForMobile/Materials/Private/PostProcessOutlines/M_SRS_Outline03.M_SRS_Outline03" :`3` "/Game/StylizedRenderingSystemForMobile/Materials/Private/PostProcessOutlines/M_SRS_Outline04.M_SRS_Outline04" :`4` "/Game/StylizedRenderingSystemForMobile/Materials/Private/PostProcessOutlines/M_SRS_Outline05.M_SRS_Outline05" :`5` "/Game/StylizedRenderingSystemForMobile/Materials/Private/PostProcessOutlines/M_SRS_Outline06.M_SRS_Outline06" :`6` "/Game/StylizedRenderingSystemForMobile/Materials/Private/PostProcessOutlines/M_SRS_Outline07.M_SRS_Outline07" :`7` "/Game/StylizedRenderingSystemForMobile/Materials/Private/PostProcessOutlines/M_SRS_Outline08.M_SRS_Outline08" :`8` "/Game/StylizedRenderingSystemForMobile/Materials/Private/PostProcessOutlines/M_SRS_Outline09.M_SRS_Outline09" :`9` "/Game/StylizedRenderingSystemForMobile/Materials/Private/PostProcessOutlines/M_SRS_Outline10.M_SRS_Outline10" :`10` "/Game/StylizedRenderingSystemForMobile/Materials/Private/PostProcessOutlines/M_SRS_Outline11.M_SRS_Outline11" :`11` "/Game/StylizedRenderingSystemForMobile/Materials/Private/PostProcessOutlines/M_SRS_Outline12.M_SRS_Outline12" :`12` "/Game/StylizedRenderingSystemForMobile/Materials/Private/PostProcessOutlines/M_SRS_Outline13.M_SRS_Outline13" :`13` "/Game/StylizedRenderingSystemForMobile/Materials/Private/PostProcessOutlines/M_SRS_Outline14.M_SRS_Outline14" :`14` "/Game/StylizedRenderingSystemForMobile/Materials/Private/PostProcessOutlines/M_SRS_Outline15.M_SRS_Outline15" :`15` "/Game/StylizedRenderingSystemForMobile/Materials/Private/PostProcessOutlines/M_SRS_Outline16.M_SRS_Outline16" :`16` "/Game/StylizedRenderingSystemForMobile/Materials/Private/PostProcessOutlines/M_SRS_Outline17.M_SRS_Outline17" :`17` "/Game/StylizedRenderingSystemForMobile/Materials/Private/PostProcessOutlines/M_SRS_Outline19.M_SRS_Outline19" :`18` "/Game/StylizedRenderingSystemForMobile/Materials/Private/PostProcessOutlines/M_SRS_Outline18.M_SRS_Outline18" :`19` "/Game/StylizedRenderingSystemForMobile/Materials/Private/PostProcessOutlines/M_SRS_Outline20.M_SRS_Outline20" :`20` "/Game/StylizedRenderingSystemForMobile/Materials/Private/PostProcessOutlines/M_SRS_Outline21.M_SRS_Outline21" :`21` "/Game/StylizedRenderingSystemForMobile/Materials/Private/PostProcessOutlines/M_SRS_Outline22.M_SRS_Outline22" :`22` "/Game/StylizedRenderingSystemForMobile/Materials/Private/PostProcessOutlines/M_SRS_Outline23.M_SRS_Outline23" :`23` "/Game/StylizedRenderingSystemForMobile/Materials/Private/PostProcessOutlines/M_SRS_Outline24.M_SRS_Outline24" :`24` "/Game/StylizedRenderingSystemForMobile/Materials/Private/PostProcessOutlines/M_SRS_Outline25.M_SRS_Outline25" :!type "MaterialInterface Object Reference")))
        (bind (_name _color _thickness _visiblewheninlineofsight_2 _visiblewhenobstructed_2 _stencilmasklow _stencilmaskhigh _advanced) (break `/Game/StylizedRenderingSystemForMobile/Blueprints/Structs/BP_SRS_Outline_Struct` _array_element))
        (`MaterialInstanceDynamic.SetVectorParameterValue` _returnvalue "Color" _color)
        (`MaterialInstanceDynamic.SetScalarParameterValue` _returnvalue "Offset Amount" _thickness)
        (bind (_mindepthdifference _obstructeddistancethreshold _opacityoverdistance _scaleoverdistance) (break `/Game/StylizedRenderingSystemForMobile/Blueprints/Structs/BP_SRS_OutlineAdvanced_Struct` _advanced))
        (`MaterialInstanceDynamic.SetScalarParameterValue` _returnvalue "Distance Threshold" _mindepthdifference)
        (`MaterialInstanceDynamic.SetScalarParameterValue` _returnvalue "Visible through Walls" (`KismetMathLibrary.Conv_BoolToDouble` _visiblewhenobstructed_2))
        (`MaterialInstanceDynamic.SetScalarParameterValue` _returnvalue "Visible LOS" (`KismetMathLibrary.Conv_BoolToDouble` _visiblewheninlineofsight_2))
        (`MaterialInstanceDynamic.SetScalarParameterValue` _returnvalue "Obstructed Depth Threshold" _obstructeddistancethreshold)
        (bind (_distancefadeinstart _distancefadeinend _distancefadeoutstart _distancefadeoutend) (break `/Game/StylizedRenderingSystemForMobile/Blueprints/Structs/BP_SRS_DistanceFade_Struct` _opacityoverdistance))
        (`MaterialInstanceDynamic.SetScalarParameterValue` _returnvalue "Distance Fade In Start" _distancefadeinstart)
        (`MaterialInstanceDynamic.SetScalarParameterValue` _returnvalue "Distance Fade In End" _distancefadeinend)
        (`MaterialInstanceDynamic.SetScalarParameterValue` _returnvalue "Distance Fade Out Start" _distancefadeoutstart)
        (`MaterialInstanceDynamic.SetScalarParameterValue` _returnvalue "Distance Fade Out End" _distancefadeoutend)
        (bind (_scalefadestart _scalefadeend _endscale) (break `/Game/StylizedRenderingSystemForMobile/Blueprints/Structs/BP_SRS_DistanceScale_Struct` _scaleoverdistance))
        (`MaterialInstanceDynamic.SetScalarParameterValue` _returnvalue "Min Distance" _scalefadestart)
        (`MaterialInstanceDynamic.SetScalarParameterValue` _returnvalue "Max Distance" _scalefadeend)
        (`MaterialInstanceDynamic.SetScalarParameterValue` _returnvalue "Distance Scale" _endscale)
        (`MaterialInstanceDynamic.SetScalarParameterValue` _returnvalue "CDS Value Min" (`KismetMathLibrary.Conv_IntToDouble` _stencilmasklow))
        (`MaterialInstanceDynamic.SetScalarParameterValue` _returnvalue "CDS Value Max" (`KismetMathLibrary.Conv_IntToDouble` _stencilmaskhigh))
        (`KismetArrayLibrary.Array_Add` (`.Array` (break `WeightedBlendables` (`.WeightedBlendables` (break `PostProcessSettings` (`PostProcessComponent.Settings` (`self.PostProcess`)))))) (make `WeightedBlendable` 1.0 _returnvalue))))))

(fn `UserConstructionScript`
  (`self.Refresh`))