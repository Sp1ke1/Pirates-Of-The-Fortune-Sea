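; Component for the mobile stylized rendering system that fakes fading shadows on registered meshes of its owning actor.
; A looping timer traces toward the active directional light, taken from the Tint actor or the first one found, and steps shadow percentage by hit result.
; It writes current and target percentages, time and interval to Custom Primitive Data, presumably for material-side interpolation.
; Initialization also writes tint, shadow intensity and rimlight, highlight and shadow scales.
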(event `self.ReceiveBeginPlay`
  (`self.Initialize`)
  (`KismetSystemLibrary.K2_SetTimerDelegate` (delegate `Update`) (`self.Time between Checks`) true))

(event `Update`
  (`self.UpdateState`))

(fn `Check Shadow`
  (returns (`In Shadow` :type Boolean))
  (bind _returnvalue (+ (`Actor.K2_GetActorLocation` (`self.GetOwner`)) (`self.Trace Offset`)))
  (bind (_outhit _returnvalue_2) (`KismetSystemLibrary.LineTraceSingle` :`Start` _returnvalue :`End` (+ _returnvalue (* (* (`Actor.GetActorForwardVector` (`self.activeLight`)) -1.0) (`self.Trace Length`))) :`TraceChannel` "TraceTypeQuery1" :`DrawTime` 0.5))
  (return _returnvalue_2))

(fn `Determine active Directional Light`
  (returns (`Directional Light` :type "DirectionalLight Object Reference") (isValid :type Boolean))
  (bind _returnvalue (`Actor.GetComponentByClass` (`GameplayStatics.GetGameMode`) "/Game/StylizedRenderingSystemForMobile/Blueprints/BP_Tint_GameModeComponent_SRS.BP_Tint_GameModeComponent_SRS_C"))
  (bind (_bp_tint_actor _is_valid) (`/Game/StylizedRenderingSystemForMobile/Blueprints/BP_Tint_GameModeComponent_SRS.Get Tint Actor` _returnvalue))
  (bind (_active_directional_light _is_valid_2) (`/Game/StylizedRenderingSystemForMobile/Blueprints/BP_Tint_SRS.Get Active Directional Light` _bp_tint_actor))
  (`/Engine/EditorBlueprintResources/StandardMacros.IsValid` _returnvalue
    (:`Is Valid`
      (if _is_valid
        (if _is_valid_2
          (bind _output_get (set `self.activeLight` _active_directional_light))
          (return _output_get true)
          (else
            _))
        (else
          (bind _outactors (`GameplayStatics.GetAllActorsOfClass` "/Script/Engine.DirectionalLight" :!label _label))
          (if (> (`KismetArrayLibrary.Array_Length` _outactors) 0)
            (bind _output (`|GetArrayItem` _outactors))
            (`/Engine/EditorBlueprintResources/StandardMacros.IsValid` _output
              (:`Is Valid`
                (bind _output_get_2 (set `self.activeLight` _output))
                (return _output_get_2 true))
              (:`Is Not Valid`
                _))))))
    (:`Is Not Valid`
      (goto _label)))
  (return null false))

(fn `Initialize`
  (bind (_tint_r _tint_g _tint_b) (break `LinearColor` (`self.Tint`)))
  (bind _fade_duration (`self.Fade Duration`))
  (bind (_directional_light _isvalid) (`self.Determine active Directional Light`))
  (if _isvalid
    (set `self.maximumChangePerStep` (`KismetMathLibrary.SelectFloat` 9999.0 (/ (`self.Time between Checks`) _fade_duration) (== _fade_duration 0.0)))
    (bind _in_shadow (`self.Check Shadow`))
    (bind _returnvalue (`KismetMathLibrary.Conv_BoolToDouble` _in_shadow))
    (set `self.Current Shadow Percentage` _returnvalue)
    (set `self.Target Shadow Percentage` _returnvalue)
    (for _array_element (`self.Meshes`)
      (`PrimitiveComponent.SetCustomPrimitiveDataVector4` _array_element 4 (`KismetMathLibrary.MakeVector4` _tint_r _tint_g _tint_b (`self.Shadow Intensity`)))
      (`PrimitiveComponent.SetCustomPrimitiveDataFloat` _array_element 8 (`self.Rimlight Size Scale`))
      (`PrimitiveComponent.SetCustomPrimitiveDataFloat` _array_element 9 (`self.Highlight Size Scale`))
      (`PrimitiveComponent.SetCustomPrimitiveDataFloat` _array_element 10 (`self.Shadow Size Scale`)))
    (else
      (`KismetSystemLibrary.PrintString` "Shadow Manager could not find Directional Light Object. If this happpened during compiling or editing of blueprints, dismiss this warning." false true (struct :`R` 0.475 :`G` 1.0 :`A` 1.0)))))

(fn `Make Mesh Dynamic`
  (params (Mesh :type "PrimitiveComponent Object Reference"))
  (`KismetArrayLibrary.Array_Add` (`self.Meshes`) Mesh)
  (`self.Initialize`)
  (`self.UpdateState`))

(fn `UpdateState`
  (bind (_directional_light _isvalid) (`self.Determine active Directional Light`))
  (if _isvalid
    (bind _in_shadow (`self.Check Shadow`))
    (set `self.Current Shadow Percentage` (`self.Target Shadow Percentage`))
    (set `self.Target Shadow Percentage` (`KismetMathLibrary.FClamp` (+ (`self.Current Shadow Percentage`) (* (`self.maximumChangePerStep`) (`KismetMathLibrary.SelectFloat` 1.0 -1.0 _in_shadow)))))
    (for _array_element (`self.Meshes`)
      (`PrimitiveComponent.SetCustomPrimitiveDataVector4` _array_element 0 (`KismetMathLibrary.MakeVector4` (`self.Current Shadow Percentage`) (`self.Target Shadow Percentage`) (`GameplayStatics.GetUnpausedTimeSeconds`) (`self.Time between Checks`))))
    (else
      (`KismetSystemLibrary.PrintString` "Could not find a Directional Light Actor." false))))