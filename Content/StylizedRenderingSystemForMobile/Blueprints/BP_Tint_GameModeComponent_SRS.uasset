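; Game mode component of the Stylized Rendering System for Mobile that provides access to the level's BP_Tint_SRS tint actor.
; GetTintActor returns the cached reference when valid, otherwise searches by class, caches the first actor found and reports whether one exists.
; The lookup is lazy, as the BeginPlay and Tick events are disabled placeholders.
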(fn `Get Tint Actor`
  (returns (`BP Tint Actor` :type "/Game/StylizedRenderingSystemForMobile/Blueprints/BP_Tint_SRS Object Reference") (`is Valid` :type Boolean))
  (bind _bp_tint_actor (`self.BP_Tint_Actor`))
  (`/Engine/EditorBlueprintResources/StandardMacros.IsValid` _bp_tint_actor
    (:`Is Valid`
      (return _bp_tint_actor true))
    (:`Is Not Valid`
      (bind _outactors (`GameplayStatics.GetAllActorsOfClass` "/Game/StylizedRenderingSystemForMobile/Blueprints/BP_Tint_SRS.BP_Tint_SRS_C"))
      (if (> (`KismetArrayLibrary.Array_Length` _outactors) 0)
        (bind _output_get (set `self.BP_Tint_Actor` (`|GetArrayItem` _outactors)))
        (return _output_get true)
        (else
          (return null false))))))