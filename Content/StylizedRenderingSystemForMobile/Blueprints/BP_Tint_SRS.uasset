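; Stylized rendering controller actor that drives global tint and time-of-day shading through the MPC_SRS material parameter collection.
; Refresh runs on construction, BeginPlay and UpdateDaytime, resetting daytime parameters and writing the base Tint.
; With daytime controls enabled, it makes Sun or Moon the atmosphere light and publishes its inverted forward vector.
; Daytime curves, blended by strength values, set highlight, rimlight and shadow opacity, scale and color, and multiply the tint.
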(event `self.ReceiveBeginPlay`
  (`self.Refresh`))

(fn `Get Active Directional Light`
  (returns (`Active Directional Light` :type "DirectionalLight Object Reference") (`is Valid` :type Boolean))
  (bind _active_directional_light (`self.Active Directional Light`))
  (`/Engine/EditorBlueprintResources/StandardMacros.IsValid` _active_directional_light
    (:`Is Valid`
      (return _active_directional_light true))
    (:`Is Not Valid`
      (bind _outactors (`GameplayStatics.GetAllActorsOfClass` "/Script/Engine.DirectionalLight"))
      (if (> (`KismetArrayLibrary.Array_Length` _outactors) 0)
        (bind _output_get (set `self.Active Directional Light` (`|GetArrayItem` _outactors)))
        (return _output_get true)
        (else
          (return null false))))))

(fn `Refresh`
  (bind _returnvalue (`KismetMathLibrary.InRange_FloatFloat` (`self.Daytime`) (`self.Sunrise Time`) (`self.Sunset Time`)))
  (bind _returnvalue_2 (select `bool` _returnvalue :`false` (`self.Moon`) :`true` (`self.Sun`)))
  (bind (_asdirectional_light_component _bsuccess) (cast `DirectionalLightComponent` (`Light.LightComponent` _returnvalue_2) :!pure true))
  (bind (_asdirectional_light_component_2 _bsuccess_2) (cast `DirectionalLightComponent` (`Light.LightComponent` (select `bool` (not _returnvalue) :`false` (`self.Moon`) :`true` (`self.Sun`))) :!pure true))
  (`self.Reset Daytime MPC`)
  (`KismetMaterialLibrary.SetVectorParameterValue` "/Game/StylizedRenderingSystemForMobile/Materials/Private/MPC_SRS.MPC_SRS" "Tint" (`self.Tint`))
  (if (`self.Enable Daytime Controls`)
    (`|ExecutionSequence`
      (:`then_0`
        ;[1 1 1] Sun / Moon Switch
        (if (and (`KismetSystemLibrary.IsValid` (`self.Moon`)) (`KismetSystemLibrary.IsValid` (`self.Sun`)))
          (if (and _bsuccess _bsuccess_2)
            (`DirectionalLightComponent.SetAtmosphereSunLight` _asdirectional_light_component true)
            (set `self.Active Directional Light` _returnvalue_2)
            (`KismetMaterialLibrary.SetVectorParameterValue` "/Game/StylizedRenderingSystemForMobile/Materials/Private/MPC_SRS.MPC_SRS" "Directional Light Vector" (`KismetMathLibrary.MakeColor` (.x (* (`SceneComponent.GetForwardVector` _asdirectional_light_component) -1.0)) (.y (* (`SceneComponent.GetForwardVector` _asdirectional_light_component) -1.0)) (.z (* (`SceneComponent.GetForwardVector` _asdirectional_light_component) -1.0))))
            (`DirectionalLightComponent.SetAtmosphereSunLight` _asdirectional_light_component_2 false))))
      (:`then_1`
        ;[1 1 1] Highlight / Rimlight Opacity
        (`KismetMaterialLibrary.SetScalarParameterValue` "/Game/StylizedRenderingSystemForMobile/Materials/Private/MPC_SRS.MPC_SRS" "Highlight / Rimlight Opacity" (`KismetMathLibrary.Lerp` 1.0 (`CurveFloat.GetFloatValue` (`self.Highlight/Rimlight Opacity by Daytime`) (`self.Daytime`)) (`self.HLRL Curve Strength`))))
      (:`then_2`
        ;[1 1 1] Shadow Opacity
        (`KismetMaterialLibrary.SetScalarParameterValue` "/Game/StylizedRenderingSystemForMobile/Materials/Private/MPC_SRS.MPC_SRS" "Shadow Opacity" (`KismetMathLibrary.Lerp` 1.0 (`CurveFloat.GetFloatValue` (`self.Shadow Opacity by Daytime`) (`self.Daytime`)) (`self.SO Curve Strength`))))
      (:`then_3`
        ;[1 1 1] Highlight / Rimlight Scale
        (`KismetMaterialLibrary.SetScalarParameterValue` "/Game/StylizedRenderingSystemForMobile/Materials/Private/MPC_SRS.MPC_SRS" "Rimlight Scale" (`KismetMathLibrary.Lerp` 1.0 (`CurveFloat.GetFloatValue` (`self.Rimlight Scale by Daytime`) (`self.Daytime`)) (`self.RL Curve Strength`)))
        (`KismetMaterialLibrary.SetScalarParameterValue` "/Game/StylizedRenderingSystemForMobile/Materials/Private/MPC_SRS.MPC_SRS" "Highlight Scale" (`KismetMathLibrary.Lerp` 1.0 (`CurveFloat.GetFloatValue` (`self.Highlight Scale by Daytime`) (`self.Daytime`)) (`self.HL Curve Strength`))))
      (:`then_4`
        ;[1 1 1] Shadow Scale
        (`KismetMaterialLibrary.SetScalarParameterValue` "/Game/StylizedRenderingSystemForMobile/Materials/Private/MPC_SRS.MPC_SRS" "Shadow Scale" (`KismetMathLibrary.Lerp` 1.0 (`CurveFloat.GetFloatValue` (`self.Shadow Scale by Daytime`) (`self.Daytime`)) (`self.S Curve Strength`))))
      (:`then_5`
        ;[1 1 1] Global Tint
        (bind _returnvalue_3 (`KismetMaterialLibrary.GetVectorParameterValue` "/Game/StylizedRenderingSystemForMobile/Materials/Private/MPC_SRS.MPC_SRS" "Tint"))
        (`KismetMaterialLibrary.SetVectorParameterValue` "/Game/StylizedRenderingSystemForMobile/Materials/Private/MPC_SRS.MPC_SRS" "Tint" (* _returnvalue_3 (`KismetMathLibrary.LinearColorLerp` (struct :`R` 1.0 :`G` 1.0 :`B` 1.0 :`A` 1.0) (`CurveLinearColor.GetLinearColorValue` (`self.Tint Curve`) (`self.Daytime`)) (`self.Tint Curve Strength`)))))
      (:`then_6`
        ;[1 1 1] Shadow Color
        (if (`self.Change Shadow Color based on Daytime?`)
          (`KismetMaterialLibrary.SetVectorParameterValue` "/Game/StylizedRenderingSystemForMobile/Materials/Private/MPC_SRS.MPC_SRS" "DT Shadow Tint" (`KismetMathLibrary.LinearColorLerp` (struct) (`CurveLinearColor.GetLinearColorValue` (`self.Shadow Color Curve`) (`self.Daytime`)) (`self.S Color Curve Brightness`)))))
      (:`then_7`
        ;[1 1 1] HLRL Color
        (if (`self.Change Highlight Color based on Daytime?`)
          (`KismetMaterialLibrary.SetVectorParameterValue` "/Game/StylizedRenderingSystemForMobile/Materials/Private/MPC_SRS.MPC_SRS" "DT HLRL Tint" (`KismetMathLibrary.LinearColorLerp` (struct) (`CurveLinearColor.GetLinearColorValue` (`self.HLRL Color Curve`) (`self.Daytime`)) (`self.HLRL Color Curve Brightness`))))))))

(fn `Reset Daytime MPC`
  (`KismetMaterialLibrary.SetVectorParameterValue` "/Game/StylizedRenderingSystemForMobile/Materials/Private/MPC_SRS.MPC_SRS" "Directional Light Vector" (make `LinearColor` 1.0 1.0 1.0))
  (`KismetMaterialLibrary.SetScalarParameterValue` "/Game/StylizedRenderingSystemForMobile/Materials/Private/MPC_SRS.MPC_SRS" "Highlight / Rimlight Opacity" 1.0)
  (`KismetMaterialLibrary.SetScalarParameterValue` "/Game/StylizedRenderingSystemForMobile/Materials/Private/MPC_SRS.MPC_SRS" "Shadow Opacity" 1.0)
  (`KismetMaterialLibrary.SetScalarParameterValue` "/Game/StylizedRenderingSystemForMobile/Materials/Private/MPC_SRS.MPC_SRS" "Rimlight Scale" 1.0)
  (`KismetMaterialLibrary.SetScalarParameterValue` "/Game/StylizedRenderingSystemForMobile/Materials/Private/MPC_SRS.MPC_SRS" "Highlight Scale" 1.0)
  (`KismetMaterialLibrary.SetScalarParameterValue` "/Game/StylizedRenderingSystemForMobile/Materials/Private/MPC_SRS.MPC_SRS" "Shadow Scale" 1.0)
  (`KismetMaterialLibrary.SetVectorParameterValue` "/Game/StylizedRenderingSystemForMobile/Materials/Private/MPC_SRS.MPC_SRS" "DT Shadow Tint" (make `LinearColor` 1.0 1.0 1.0))
  (`KismetMaterialLibrary.SetVectorParameterValue` "/Game/StylizedRenderingSystemForMobile/Materials/Private/MPC_SRS.MPC_SRS" "DT HLRL Tint" (make `LinearColor` 1.0 1.0 1.0)))

(fn `Update Daytime`
  (params (Daytime :type "Float (double-precision)"))
  (set `self.Daytime` Daytime)
  (`self.Refresh`))

(fn `UserConstructionScript`
  (`self.Refresh`))